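; BP_TimeFloor is a floor actor that destroys itself shortly after the player character steps on it.
; BoxCollider's begin overlap casts to BP_ThirdPersonCharacter and calls TimerEvent, which waits on a short Delay before destroying the actor.
; End overlap resets a Timer variable that TimerEvent never reads, so leaving does not cancel the destruction.
; Debug strings print on overlaps and timer start.
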(event `TimerEvent`
  (`KismetSystemLibrary.PrintString` "Call!")
  (`KismetSystemLibrary.Delay` 2.0)
  (`self.K2_DestroyActor`))

(event `self.BoxCollider.OnComponentBeginOverlap`
  (params (OverlappedComponent :type "PrimitiveComponent Object Reference") (OtherActor :type "Actor Object Reference") (OtherComp :type "PrimitiveComponent Object Reference") (OtherBodyIndex :type Integer) (bFromSweep :type Boolean) (SweepResult :type "HitResult Structure (by ref)"))
  (`KismetSystemLibrary.PrintString` "in")
  (cast `/Game/ThirdPerson/Blueprints/BP_ThirdPersonCharacter` OtherActor)
  (`self.TimerEvent`))

(event `self.BoxCollider.OnComponentEndOverlap`
  (params (OverlappedComponent :type "PrimitiveComponent Object Reference") (OtherActor :type "Actor Object Reference") (OtherComp :type "PrimitiveComponent Object Reference") (OtherBodyIndex :type Integer))
  (`KismetSystemLibrary.PrintString` "in")
  (cast `/Game/ThirdPerson/Blueprints/BP_ThirdPersonCharacter` OtherActor)
  (set `self.Timer` 0.0))

(fn `UserConstructionScript`)