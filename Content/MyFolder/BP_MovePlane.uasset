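; BP_MovePlane is an actor that moves a plane mesh back and forth along a spline.
; Each tick it advances a Distance value by Speed times delta time and places the plane at that world-space point on the spline.
; When Distance passes either end of the spline, Speed flips sign to reverse direction.
; Only position is updated; rotation is left unchanged and movement does not sweep.
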(event `self.ReceiveTick`
  (params (DeltaSeconds :type "Float (single-precision)"))
  (bind _output_get (set `self.Distance` (+ (* DeltaSeconds (`self.Speed`)) (`self.Distance`))))
  (if (or (> _output_get (`SplineComponent.GetSplineLength` (`self.Spline`))) (< _output_get 0.0))
    (set `self.Speed` (* (`self.Speed`) -1.0)))
  (`SceneComponent.K2_SetWorldLocation` (`self.Plane`) (`SplineComponent.GetLocationAtDistanceAlongSpline` (`self.Spline`) _output_get "World") false false))

(fn `UserConstructionScript`)